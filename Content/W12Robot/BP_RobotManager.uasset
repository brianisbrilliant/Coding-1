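; BP_RobotManager advances the robot simulation by one day each time the StartNewDay input (key 1) is pressed.
; It enables input from player controller 0 on BeginPlay.
; On each press it finds every BP_Robot, decrements its Charge, then calls its Status and Move functions.
; It prints each robot's name and X/Y position on screen after the move.
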(event EventBeginPlay
  (Input|EnableInput (Game|GetPlayerController 0)))

(event Input|ActionEvents|InputActionStartNewDay
  (params (Key :type Key%20Structure :default "None"))
  ;[1 1 1] Comment
  (:Pressed
    (bind _outactors (Actor|GetAllActorsOfClass "/Game/W12Robot/BP_Robot.BP_Robot_C"))
    (for _array_element _outactors
      (Math|Integer|DecrementInt (Variables|/Game/W12Robot/BP_Robot.BP_Robot_C|GetCharge _array_element)
        (:%20%20
          (Default|Status _array_element)
          (Default|Move _array_element)
          (Development|PrintString (Utilities|String|Append (Variables|/Game/W12Robot/BP_Robot.BP_Robot_C|GetName _array_element) "Pos: " (Utilities|String|ToString(Float) (.x (.location (Transformation|GetActorTransform _array_element)))) "," (Utilities|String|ToString(Float) (.y (.location (Transformation|GetActorTransform _array_element))))) true true "(R=1.000000,G=0.583200,B=0.000000,A=1.000000)" 4.0))))))

(fn ConstructionScript)