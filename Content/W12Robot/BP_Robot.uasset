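; Robot actor that wanders a bounded grid, spending charge as it moves and sharing it with depleted robots.
; BeginPlay randomizes unset name and charge, then loops each second, calling Move for a random clamped XY step while charge remains.
; Status prints the charge and colors the head green or red.
; Sphere overlap transfers charge to an empty robot when this one has enough surplus; the timed self-recharge branch is disconnected.
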(event OnComponentBeginOverlap(SphereCollision)
  (params (OverlappedComponent :type Primitive%20Component%20Object%20Reference) (OtherActor :type Actor%20Object%20Reference) (OtherComp :type Primitive%20Component%20Object%20Reference) (OtherBodyIndex :type Integer) (bFromSweep :type Boolean) (SweepResult :type Hit%20Result%20Structure%20%28by%20ref%29))
  (bind _asbp_robot (Utilities|Casting|CastToBP_Robot OtherActor)) ; is the other thing a robot?
  (if (< (Variables|BP_Robot_C|GetCharge _asbp_robot) 1) ; True if robot's charge is 0.
    (if (> (Variables|Default|GetCharge) 10) ; True if this robot has more than 10 charge.
      (Variables|BP_Robot_C|SetCharge _asbp_robot 10) ; other robot
      (Variables|Default|SetCharge (- (Variables|Default|GetCharge) 10)) ; This robot
      (Development|PrintString "CHARGING CHARGING CHARGING" true true "(R=1.000000,G=0.000000,B=0.855670,A=1.000000)" 5.0)
      (CallFunction|Status _asbp_robot))))

(event Custom|Status
  (bind _head (Variables|Default|Gethead))
  (if (> (Variables|Default|GetCharge) 0)
    (Development|PrintString (Utilities|String|Append "Robot \"" (Variables|Default|GetName) "\" has a charge of " (Utilities|String|ToString(Integer) (Variables|Default|GetCharge)) ".") true true "(R=0.117491,G=1.000000,B=0.350779,A=1.000000)" 1e+01)
    (Rendering|Material|SetMaterial _head 0 "/Game/W12Robot/Green.Green")
    (else
      (Variables|Default|SetCharge 0)
      (Development|PrintString (Utilities|String|Append "Robot \"" (Variables|Default|GetName) "\" has a charge of " (Utilities|String|ToString(Integer) (Variables|Default|GetCharge)) ".") true true "(R=1.000000,G=0.064546,B=0.072504,A=1.000000)" 1e+01)
      (Rendering|Material|SetMaterial _head 0 "/Game/W12Robot/Red.Red"))))

(event Custom|Move
  (bind _returnvalue (Transformation|GetActorLocation))
  (Transformation|SetActorLocation (+ (Transformation|GetActorLocation) (Math|Vector|MakeVector (* (Math|Random|RandomIntegerinRange -1 1) 100) (* (Math|Random|RandomIntegerinRange -1 1) 100) 0.0)) false false)
  (Math|Integer|DecrementInt (Variables|Default|GetCharge)
    (:%20%20
      (if (> (.x _returnvalue) 5e+02)
        (Transformation|SetActorLocation (Math|Vector|MakeVector 5e+02 (.y _returnvalue) (.z _returnvalue)) false false))
      (if (< (.x _returnvalue) -5e+02)
        (Transformation|SetActorLocation (Math|Vector|MakeVector -5e+02 (.y _returnvalue) (.z _returnvalue)) false false))
      (if (> (.y _returnvalue) 5e+02)
        (Transformation|SetActorLocation (Math|Vector|MakeVector (.x _returnvalue) 5e+02 (.z _returnvalue)) false false))
      (if (< (.y _returnvalue) -5e+02)
        (Transformation|SetActorLocation (Math|Vector|MakeVector (.x _returnvalue) -5e+02 (.z _returnvalue)) false false))
      (CallFunction|Status) ; This is the end of the move function
    )))

(event EventBeginPlay
  ;[1 1 1] Randomize Charge if not set
  (if (== (Variables|Default|GetCharge) -1)
    (Variables|Default|SetCharge (Math|Random|RandomIntegerinRange 4 10)))
  ;[1 1 1] Randomize Name if not set
  (if (Utilities|Enum|Equal(Enum) (Variables|Default|GetName) "Robot")
    (Variables|Default|SetName (.OutItem (Utilities|Array|Random (Variables|Default|GetRobotNames)))))
  (CallFunction|Status)
  (if (> (Variables|Default|GetCharge) 0) :!label _label
    (CallFunction|Move))
  (Utilities|FlowControl|Delay 1.0)
  (goto _label))

(fn ConstructionScript)