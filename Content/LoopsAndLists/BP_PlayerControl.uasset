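; BP_PlayerControl is an input-handling Blueprint that destroys one enemy per left mouse click.
; On BeginPlay it enables input from player controller 0 and finds the BP_EnemySpawner in the level.
; Each click gathers all BP_Enemy actors and, if any exist, destroys the first in the array and decrements the spawner's EnemyCount.
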(event EventBeginPlay
  (Input|EnableInput (Game|GetPlayerController 0))
  (bind _returnvalue (Actor|GetActorOfClass "/Game/LoopsAndLists/BP_EnemySpawner.BP_EnemySpawner_C")))

(event Input|MouseEvents|LeftMouseButton
  (params (Key :type Key%20Structure :default "None"))
  (:Pressed
    (bind _outactors (Actor|GetAllActorsOfClass "/Game/LoopsAndLists/BP_Enemy.BP_Enemy_C"))
    (if (> (Utilities|Array|Length _outactors) 0) ; Make sure at least 1 enemy exists
      (Actor|DestroyActor (Utilities|Array|Get(acopy) _outactors))
      (Math|Integer|DecrementInt (Variables|/Game/LoopsAndLists/BP_EnemySpawner.BP_EnemySpawner_C|GetEnemyCount (stale EventBeginPlay _returnvalue))))))

(fn ConstructionScript)