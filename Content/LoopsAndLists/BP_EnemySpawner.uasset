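; BP_EnemySpawner spawns randomly named enemies in waves at the level's BP_EnemySpawnPoint actors.
; On BeginPlay it shuffles the spawn points, then walks through them in a delayed loop, spawning while EnemyCount is below MaxEnemies.
; After the last point it polls until EnemyCount reaches zero, then increments the wave, reshuffles and repeats.
; EnemyCount is only incremented here, and the AllEnemies tracking is unconnected TODO code.
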(event EventBeginPlay
  ;[0.6098 0.1042 1] Get Spawn Points array
  (bind _outactors (Actor|GetAllActorsOfClass "/Game/LoopsAndLists/BP_EnemySpawnPoint.BP_EnemySpawnPoint_C"))
  (bind _output_get (Variables|Default|SetSpawnPoints _outactors))
  (Utilities|Array|Shuffle _output_get)
  (Development|PrintString (Utilities|String|Append "There are " (Utilities|String|ToString(Integer) (Utilities|Array|Length _output_get)) " spawn points."))
  (if (< (Variables|Default|GetEnemyCount) (Variables|Default|GetMaxEnemies)) :!label _label
    (bind _returnvalue (Game|SpawnActorfromClass "/Game/LoopsAndLists/BP_Enemy.BP_Enemy_C" (Transformation|GetActorTransform (Utilities|Array|Get(acopy) (Variables|Default|GetSpawnPoints) (Variables|Default|GetSpawnIndex))) "Undefined" 0 0))
    ;[1 1 1] Give enemy a random Name/
    (Rendering|Components|TextRender|SetText (Variables|/Game/LoopsAndLists/BP_Enemy.BP_Enemy_C|GetTextRender _returnvalue) (Utilities|Text|ToText(String) (.OutItem (Utilities|Array|Random (Variables|Default|GetNames)))))
    (Math|Integer|IncrementInt (Variables|Default|GetEnemyCount)
      (:%20%20
        (bind _result (Math|Integer|IncrementInt (Variables|Default|GetSpawnIndex))
          (:%20%20
            ;[1 1 1] Shuffle the list if we get to the end
            (if (< _result (Utilities|Array|Length (Variables|Default|GetSpawnPoints)))
              _
              (else
                ;[1 1 1] Wait until all enemies are destroyed before building new ones.
                (if (<= (Variables|Default|GetEnemyCount) 0) :!label _label_2
                  (Variables|Default|SetSpawnIndex 0)
                  (bind _result_2 (Math|Integer|IncrementInt (Variables|Default|GetWaveCount))
                    (:%20%20
                      (Utilities|Array|Shuffle (Variables|Default|GetSpawnPoints))
                      (Development|PrintString (Utilities|String|Append "Wave " (Utilities|String|ToString(Integer) _result_2)) true true "(R=0.078316,G=0.146036,B=1.000000,A=1.000000)" 4.0)))
                  (else
                    (Utilities|FlowControl|Delay 0.2)
                    (goto _label_2))))))))))
  (Utilities|FlowControl|Delay (Variables|Default|GetDelayDuration))
  (goto _label))

(fn ConstructionScript)