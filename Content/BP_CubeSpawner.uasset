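; Cube spawner actor that spawns a series of actors at the world transform of its Cube component.
; BeginPlay optionally randomizes the spawn delay once, then prints it.
; A wired-back Delay loop logs and spawns on each pass, incrementing a counter and repeating while it is below MaxCubes.
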(event EventBeginPlay
  (if (Variables|Default|GetRandomizeDelay)
    (Variables|Default|SetDelay (Math|Random|RandomFloatinRange 0.3 0.8)))
  (Development|PrintString (Utilities|String|ToString(Float) (Variables|Default|GetDelay)) true true "(R=1.000000,G=0.900236,B=0.239883,A=1.000000)" 5.0)
  (Utilities|FlowControl|Delay (Variables|Default|GetDelay) :!label _label)
  (Development|PrintString "Spawning a cube...")
  (Game|SpawnActorfromClass "/Game/BP_ChamferCube.BP_ChamferCube_C" (Transformation|GetWorldTransform (Variables|Default|GetCube)) "Undefined" 0 0)
  (bind _result (Math|Integer|IncrementInt (Variables|Default|GetTotalCubes)) ; add 1 to totalCubes
    (:%20%20
      (if (< _result (Variables|Default|GetMaxCubes)) ; if there are less than Max Cubes, keep looping
        (goto _label)))))

(fn ConstructionScript)